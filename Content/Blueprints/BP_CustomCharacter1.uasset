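; BP_CustomCharacter1 is a player-controlled character with basic movement, a starting health value and overlap detection for interactive triggers.
; AxisX and AxisY share one SetDeltaMove call that writes an axis value to both X and Y of DeltaMove.
; Each Tick, DoMovement applies nonzero DeltaMove along the actor's forward and right vectors.
; InteractRange overlaps only print whether the other actor casts to BP_InteractiveTrigger, and BeginPlay prints the initialized MaxHealth.
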(event OnComponentBeginOverlap(InteractRange)
  (params (OverlappedComponent :type Primitive%20Component%20Object%20Reference) (OtherActor :type Actor%20Object%20Reference) (OtherComp :type Primitive%20Component%20Object%20Reference) (OtherBodyIndex :type Integer) (bFromSweep :type Boolean) (SweepResult :type Hit%20Result%20Structure%20%28by%20ref%29))
  (Utilities|Casting|CastToBP_InteractiveTrigger OtherActor
    (:then
      (Development|PrintString "Overlap Detected"))
    (:CastFailed
      (Development|PrintString "other actor casting failed" true true "(R=1.000000,G=0.071486,B=0.000000,A=1.000000)"))))

(event EventBeginPlay
  (bind _output_get (Variables|Default|SetMaxHealth (Variables|Default|GetStartingHealth)))
  (Development|PrintString (Utilities|String|Append "Health is set to:" (Utilities|String|ToString(Integer) _output_get))))

(event EventTick
  (params (DeltaSeconds :type Float%20%28single-precision%29))
  (CallFunction|DoMovement))

(event Input|AxisEvents|InputAxisAxisX
  (params (AxisValue :type Float%20%28single-precision%29))
  (CallFunction|SetDeltaMove false (Math|Vector|MakeVector AxisValue (stale Input|AxisEvents|InputAxisAxisY AxisValue) 0.0)))

(event Input|AxisEvents|InputAxisAxisY
  (params (AxisValue :type Float%20%28single-precision%29))
  (CallFunction|SetDeltaMove false (Math|Vector|MakeVector (stale Input|AxisEvents|InputAxisAxisX AxisValue) AxisValue 0.0)))

(fn ConstructionScript)

(fn SetDeltaMove
  (params (DebugMode :type Boolean) (NewDeltaMove :type Vector))
  (bind _output_get (Variables|Default|SetDeltaMove NewDeltaMove))
  (if DebugMode
    (Development|PrintString (Utilities|String|Append "New delta move is:" (Utilities|String|ToString(Vector) _output_get)))))

(fn DoMovement
  (bind _deltamove (Variables|Default|GetDeltaMove))
  (if (CallFunction|CheckifMoving)
    (Pawn|Input|AddMovementInput (Transformation|GetActorForwardVector) (.x _deltamove) false)
    (Pawn|Input|AddMovementInput (Transformation|GetActorRightVector) (.y _deltamove) false)))

(fn CheckifMoving
  (bind _deltamove (Variables|Default|GetDeltaMove))
  (return (Math|Boolean|ORBoolean (!= (.x _deltamove) 0.0) (!= (.y _deltamove) 0.0) (!= (.z _deltamove) 0.0))))