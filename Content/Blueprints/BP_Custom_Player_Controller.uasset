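; Player controller that provides click-and-drag camera rotation alongside a mouse-usable HUD.
; BeginPlay sets Game and UI input mode focused on the game mode's HUD widget.
; While PrimaryAction is held, mouse X adds yaw to the player character and mouse Y sets the spring arm's relative pitch from its target rotation, zeroing roll and yaw.
; A note on the mouse Y handler questions whether it rotates.
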(event EventBeginPlay
  (bind _asbp_game_mode_default (Utilities|Casting|CastToBP_GameModeDefault (Game|GetGameMode)))
  (Input|SetInputModeGameandUI (Game|GetPlayerController 0) (Variables|/Game/Blueprints/BP_GameModeDefault.BP_GameModeDefault_C|GetHUD _asbp_game_mode_default) "DoNotLock" false))

(event Input|ActionEvents|InputActionPrimaryAction
  (params (Key :type Key%20Structure :default "None"))
  (:Pressed
    (Variables|Default|SetLMBIsDown true))
  (:Released
    (Variables|Default|SetLMBIsDown false)))

(event Input|MouseEvents|MouseX
  (params (AxisValue :type Float%20%28single-precision%29))
  ;[1 1 1] Not Rotating???
  (if (Variables|Default|GetLMBIsDown)
    (Pawn|Input|AddControllerYawInput (Game|GetPlayerCharacter 0) AxisValue)))

(event Input|MouseEvents|MouseY
  (params (AxisValue :type Float%20%28single-precision%29))
  ;[1 1 1] Not Rotating???
  (if (Variables|Default|GetLMBIsDown)
    (bind _asbp_custom_character_1 (Utilities|Casting|CastToBP_CustomCharacter1 (Game|GetPlayerCharacter 0)))
    (bind _output_get (Variables|Default|SetCurrentPlayerCameraArm (Variables|/Game/Blueprints/BP_CustomCharacter1.BP_CustomCharacter1_C|GetSpringArm _asbp_custom_character_1)))
    (Transformation|SetRelativeRotation _output_get (Math|Rotator|MakeRotator 0.0 (+ (.pitch (Class|SpringArmComponent|GetTargetRotation _output_get)) AxisValue) 0.0) false false)))

(fn ConstructionScript)